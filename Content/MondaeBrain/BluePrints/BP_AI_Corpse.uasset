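; Corpse AI pawn that chases BP_Wolf when it sees one and otherwise wanders.
; PawnSensing sightings set CanSeeEnemy and start an AI move toward the wolf, while a short retriggerable delay clears the flag once sightings stop.
; While the flag is clear, Tick waits a random few seconds, then moves to a random reachable point around its current location.
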(event OnSeePawn(PawnSensing)
  (params (Pawn :type Pawn%20Object%20Reference))
  (bind _asbp_wolf (Utilities|Casting|CastToBP_Wolf Pawn))
  (Utilities|FlowControl|Sequence
    (:then_0
      (Variables|Default|SetcanSeeEnemy? true)
      (AI|AIMoveTo self "0, 0, 0" _asbp_wolf 5.0 false))
    (:then_1
      (Utilities|FlowControl|RetriggerableDelay 0.2)
      (Variables|Default|SetcanSeeEnemy? false))))

(event EventBeginPlay)

(event Collision|EventActorBeginOverlap
  (params (OtherActor :type Actor%20Object%20Reference)))

(event EventTick
  (params (DeltaSeconds :type Float%20%28single-precision%29))
  (if (not (Variables|Default|GetcanSeeEnemy?))
    (Utilities|FlowControl|Delay (Math|Random|RandomFloatinRange 2.0 5.0))
    (AI|AIMoveTo self (.RandomLocation (AI|Navigation|GetRandomReachablePointinRadius (Transformation|GetActorLocation) 3e+03 0 0)) 0 5.0 false)))

(fn ConstructionScript)